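; Player character that acts as a free-fly camera and actor picker, adding the SP_UMG_Menu widget on begin play.
; Mouse axes drive camera yaw and clamped pitch, while input axes offset the actor along the view, sideways or vertically, with wheel-adjusted speed for planar moves.
; Either Ctrl key toggles between game-only and cursor-visible UI input modes.
; Left click passes the actor under the cursor to the game instance's WorldActorsManager for selection.
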(event EventBeginPlay
  (bind _returnvalue (Game|GetPlayerController 0))
  (bind _cameracomponent (Variables|Default|GetCameraComponent))
  (bind _relativerotation (Variables|/Script/Engine.SceneComponent|GetRelativeRotation _cameracomponent))
  ;[1 0.9341 0.8498] Begin Play
  (Variables|Default|SetCameraYaw (.yaw _relativerotation))
  (Variables|Default|SetCameraPitch (.pitch _relativerotation))
  (Development|ExecuteConsoleCommand "r.Streaming.PoolSize 20000" 0)
  ;;[0.08333 0.07552 0.07552] Input Mode Game and UI
  (Input|SetInputModeGameOnly _returnvalue)
  (Variables|/Script/Engine.PlayerController|SetbShowMouseCursor _returnvalue true)
  (Input|SetInputModeGameandUI _returnvalue 0 "DoNotLock" true)
  (bind _returnvalue_2 (UserInterface|CreateWidget "/Game/New/Blueprints/UI/SP_UMG_Menu.SP_UMG_Menu_C"))
  (bind _output_get (Variables|Default|SetMenu%20Widget _returnvalue_2))
  (UserInterface|Viewport|AddtoViewport _output_get 0))

(event Collision|EventActorBeginOverlap
  (params (OtherActor :type Actor%20Object%20Reference)))

(event EventTick
  (params (DeltaSeconds :type Float%20%28single-precision%29)))

(event Input|AxisEvents|InputAxisMoveForward
  (params (AxisValue :type Float%20%28single-precision%29))
  ;[1 1 1] Move Forward
  (CallFunction|MoveForward (* AxisValue (Variables|Default|GetMovementSpeed))))

(event Input|AxisEvents|InputAxisMoveRight
  (params (AxisValue :type Float%20%28single-precision%29))
  ;[1 1 1] Move Right
  (CallFunction|MoveRight (* AxisValue (Variables|Default|GetMovementSpeed))))

(event Input|AxisEvents|InputAxisTilt
  (params (AxisValue :type Float%20%28single-precision%29))
  ;[1 1 1] Tilt
  (CallFunction|Tilt AxisValue))

(event Input|MouseEvents|MouseWheelAxis
  (params (AxisValue :type Float%20%28single-precision%29))
  ;[1 1 1] Change Movement Speed
  (Variables|Default|SetMovementSpeed (Math|Float|Clamp(Float) (+ (Variables|Default|GetMovementSpeed) (* AxisValue 0.01)) 0.01 (Variables|Default|GetMaximumMovementSpeed))))

(event Input|MouseEvents|MouseX
  (params (AxisValue :type Float%20%28single-precision%29))
  ;[1 1 1] Turn And LookUp
  (Variables|Default|SetCameraYaw (+ (Variables|Default|GetCameraYaw) AxisValue 0.0))
  (Transformation|SetRelativeRotation (Variables|Default|GetCameraComponent) (Math|Rotator|MakeRotator 0.0 (Variables|Default|GetCameraPitch) (Variables|Default|GetCameraYaw)) false false))

(event Input|MouseEvents|MouseY
  (params (AxisValue :type Float%20%28single-precision%29))
  ;[1 1 1] Turn And LookUp
  (Variables|Default|SetCameraPitch (Math|Float|Clamp(Float) (+ (Variables|Default|GetCameraPitch) AxisValue) -8e+01 8e+01))
  (Transformation|SetRelativeRotation (Variables|Default|GetCameraComponent) (Math|Rotator|MakeRotator 0.0 (Variables|Default|GetCameraPitch) (Variables|Default|GetCameraYaw)) false false))

(event Input|MouseEvents|LeftMouseButton
  (params (Key :type Key%20Structure :default "None"))
  (:Pressed
    (bind _objecthit (Class|RuntimeFBXImportBPLibrary|CheckHitatMouseCursor))
    (bind _asspgame_instance (Utilities|Casting|CastToSPGameInstance (Game|GetGameInstance)))
    (bind _returnvalue (Class|SPGameInstance|GetWorldActorsManager _asspgame_instance))
    (Class|WorldActorsManager|DoUnSelect _returnvalue)
    (Variables|/Script/FBXImportDemo.WorldActorsManager|Setm_pSelectedActor _returnvalue (.HitActor (Collision|BreakHitResult _objecthit)))
    (Class|WorldActorsManager|DoSelect _returnvalue)))

(event Input|KeyboardEvents|RightCtrl
  (params (Key :type Key%20Structure :default "None"))
  (bind _returnvalue (Game|GetPlayerController 0))
  ;[1 1 1] Toggle Input Mode
  (:Pressed
    (if (Variables|Default|GetIsFlyCamMode)
      (Variables|Default|SetIsFlyCamMode false)
      (Variables|/Script/Engine.PlayerController|SetbShowMouseCursor _returnvalue true)
      (Input|SetInputModeGameandUI _returnvalue 0 "DoNotLock" true)
      (else
        (Variables|Default|SetIsFlyCamMode true)
        (Variables|/Script/Engine.PlayerController|SetbShowMouseCursor _returnvalue false)
        (Input|SetInputModeGameOnly _returnvalue)))))

(event Input|KeyboardEvents|LeftCtrl
  (params (Key :type Key%20Structure :default "None"))
  (bind _returnvalue (Game|GetPlayerController 0))
  ;[1 1 1] Toggle Input Mode
  (:Pressed
    (if (Variables|Default|GetIsFlyCamMode)
      (Variables|Default|SetIsFlyCamMode false)
      (Variables|/Script/Engine.PlayerController|SetbShowMouseCursor _returnvalue true)
      (Input|SetInputModeGameandUI _returnvalue 0 "DoNotLock" true)
      (else
        (Variables|Default|SetIsFlyCamMode true)
        (Variables|/Script/Engine.PlayerController|SetbShowMouseCursor _returnvalue false)
        (Input|SetInputModeGameOnly _returnvalue)))))

(fn ConstructionScript)

(fn MoveForward
  (params (Value :type Float%20%28single-precision%29))
  (bind _cameracomponent (Variables|Default|GetCameraComponent))
  (if (!= Value 0.0)
    (Transformation|AddActorLocalOffset (* (Math|Vector|GetForwardVector (Math|Rotator|FindLookatRotation (Transformation|GetWorldLocation (Variables|Default|GetCameraComponent)) (+ (Transformation|GetWorldLocation _cameracomponent) (* (Math|Vector|GetForwardVector (Variables|/Script/Engine.SceneComponent|GetRelativeRotation _cameracomponent)) 5e+03)))) (* Value (Variables|Default|GetFlySpeed))) false false)))

(fn MoveRight
  (params (Value :type Float%20%28single-precision%29))
  (bind _cameracomponent (Variables|Default|GetCameraComponent))
  (bind _relativerotation (Variables|/Script/Engine.SceneComponent|GetRelativeRotation _cameracomponent))
  (bind _returnvalue (Math|Rotator|MakeRotator 0.0 0.0 (.yaw _relativerotation)))
  (bind _returnvalue_2 (Math|Vector|GetForwardVector _returnvalue))
  (if (!= Value 0.0)
    (Transformation|AddActorLocalOffset (* (Math|Vector|MakeVector (* (.y _returnvalue_2) -1.0) (.x _returnvalue_2) 0.0) (* Value (Variables|Default|GetPanSpeed))) false false)))

(fn Tilt
  (params (Value :type Float%20%28single-precision%29))
  (Transformation|AddActorLocalOffset (Math|Vector|MakeVector 0.0 0.0 (* Value (Variables|Default|GetTiltSpeed))) false false))